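; Boss javelin attack actor that turns to face the player each tick until launched.
; LaunchAttack tilts the mesh, stops tracking, then traces toward the player's offset position to pick an impact point marked with a fading decal.
; After a one-second warning it eases the root to that point, shakes the camera and calls FadeOut.
; A missed trace halts the launch, and the trace's debug draw is still enabled.
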(event `self.ReceiveBeginPlay`
  (`parent.ReceiveBeginPlay`))

(event `self.ReceiveTick`
  (params (DeltaSeconds :type "Float (single-precision)"))
  (bind (_returnvalue_roll _returnvalue_pitch _returnvalue_yaw) (`KismetMathLibrary.BreakRotator` (`KismetMathLibrary.FindLookAtRotation` (`self.K2_GetActorLocation`) (`self.K2_GetActorLocation` (`GameplayStatics.GetPlayerCharacter` 0)))))
  (`self.K2_SetActorRotation` (`KismetMathLibrary.MakeRotator` 0.0 0.0 _returnvalue_yaw)))

(event `self.LaunchAttack`
  (bind _returnvalue (`GameplayStatics.GetPlayerCharacter` 0))
  (bind _staticmesh (`self.StaticMesh`))
  (bind _defaultsceneroot (`self.DefaultSceneRoot`))
  (`KismetSystemLibrary.MoveComponentTo` _staticmesh (`SceneComponent.RelativeLocation` _staticmesh) (struct :`Yaw` 90.0 :`Roll` 90.0) true true)
  (`KismetSystemLibrary.Delay` 0.2)
  (`self.SetActorTickEnabled` false)
  (bind _output_get (set `self.Target` (+ (`self.K2_GetActorLocation` _returnvalue) (`self.offset`))))
  (bind (_outhit _returnvalue_2) (`KismetSystemLibrary.LineTraceSingle` (`self.K2_GetActorLocation`) _output_get "TraceTypeQuery2" false (`|MakeArray` _returnvalue :!type "Actor Object Reference") "ForDuration"))
  (if _returnvalue_2
    (set `self.Target` (`.Location` (`GameplayStatics.BreakHitResult` _outhit)))
    (bind _returnvalue_3 (`GameplayStatics.SpawnDecalAtLocation` "/Game/MyAssets/Boss/decal/BT_Decal.BT_Decal" (150.0 150.0 150.0) (`self.Target`) (struct :`Pitch` -90.0) 4.0))
    (`DecalComponent.SetFadeIn` _returnvalue_3 0.0 1.0)
    (`DecalComponent.SetFadeOut` _returnvalue_3 1.0 1.0 true)
    (`KismetSystemLibrary.Delay` 1.0)
    (`KismetSystemLibrary.MoveComponentTo` _defaultsceneroot (`self.Target`) (`SceneComponent.RelativeRotation` _defaultsceneroot) true true)
    (`GameplayStatics.PlayWorldCameraShake` "/Game/MyAssets/Boss/CameraShake_Attack.CameraShake_Attack_C" (0.0 0.0 0.0) 500.0 5000.0)
    (`KismetSystemLibrary.Delay` 1.0)
    (`self.Fade Out`)))

(fn `UserConstructionScript`
  (`parent.UserConstructionScript`))