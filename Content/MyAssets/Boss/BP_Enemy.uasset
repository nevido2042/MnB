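; Boss enemy character that detects MnBCharacters with a sphere and offers two attacks against a target.
; Sphere overlaps set or clear the AI Blackboard "Target" key, whose value is printed every tick for debugging.
; ATK_01 turns to the target and plays a random montage.
; ATK_02 turns, leaps opposite the player's camera forward, plays a montage and uses delays to toggle jump and attack-active flags.
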(event `self.SphereVision.OnComponentBeginOverlap`
  (params (OverlappedComponent :type "PrimitiveComponent Object Reference") (OtherActor :type "Actor Object Reference") (OtherComp :type "PrimitiveComponent Object Reference") (OtherBodyIndex :type Integer) (bFromSweep :type Boolean) (SweepResult :type "HitResult Structure (by ref)"))
  ;[1 1 1] Set Target/Get Target/ClearTarget
  (if (!= OtherActor self)
    (bind _asmn_bcharacter (cast `MnBCharacter` OtherActor))
    (`self.SetTarget` _asmn_bcharacter)))

(event `self.SphereVision.OnComponentEndOverlap`
  (params (OverlappedComponent :type "PrimitiveComponent Object Reference") (OtherActor :type "Actor Object Reference") (OtherComp :type "PrimitiveComponent Object Reference") (OtherBodyIndex :type Integer))
  ;[1 1 1] Set Target/Get Target/ClearTarget
  (if (== OtherActor (`self.GetTarget`))
    (`self.ClearTarget`)))

(event `self.ReceiveTick`
  (params (DeltaSeconds :type "Float (single-precision)"))
  ;[1 1 1] Set Target/Get Target/ClearTarget
  (`KismetSystemLibrary.PrintString` (`KismetStringLibrary.Concat_StrStr` "CurTarget" (`KismetSystemLibrary.GetDisplayName` (`self.GetTarget`)))))

(event `ATK_01`
  (params (Target :type "Actor Object Reference"))
  (bind (_returnvalue_roll _returnvalue_pitch _returnvalue_yaw) (`KismetMathLibrary.BreakRotator` (`KismetMathLibrary.FindLookAtRotation` (`self.K2_GetActorLocation`) (`self.K2_GetActorLocation` Target))))
  (`|ExecutionSequence`
    (:`then_0`
      (`/Engine/EditorBlueprintResources/StandardMacros.IsValid` Target
        (:`Is Valid`
          (`self.K2_SetActorRotation` (`KismetMathLibrary.MakeRotator` 0.0 0.0 _returnvalue_yaw)))))
    (:`then_1`
      (`|PlayMontage` (`self.Mesh`) (`|GetArrayItem` (`self.AttackArray`) (`KismetMathLibrary.RandomIntegerInRange` 0 1))))))

(event `ATK_02`
  (params (Target :type "Actor Object Reference"))
  (bind (_returnvalue_roll _returnvalue_pitch _returnvalue_yaw) (`KismetMathLibrary.BreakRotator` (`KismetMathLibrary.FindLookAtRotation` (`self.K2_GetActorLocation`) (`self.K2_GetActorLocation` Target))))
  (`|ExecutionSequence`
    (:`then_0`
      (`/Engine/EditorBlueprintResources/StandardMacros.IsValid` Target
        (:`Is Valid`
          (`self.K2_SetActorRotation` (`KismetMathLibrary.MakeRotator` 0.0 0.0 _returnvalue_yaw)))))
    (:`then_1`
      (set `self.IsJumping` true)
      (bind _asmn_bcharacter (cast `MnBCharacter` (`GameplayStatics.GetPlayerCharacter` 0)))
      (bind (_returnvalue_x _returnvalue_y) (`KismetMathLibrary.BreakVector` (`SceneComponent.GetForwardVector` (`MnBCharacter.FollowCamera` _asmn_bcharacter))))
      (`self.LaunchCharacter` (`KismetMathLibrary.MakeVector` (* _returnvalue_x -500.0) (* _returnvalue_y -500.0) 900.0) true true)
      (`|PlayMontage` (`self.Mesh`)
        (:`then`
          (`KismetSystemLibrary.Delay` 0.8)
          (set `self.IsJumping` false)
          (`KismetSystemLibrary.Delay` 0.4)
          (set `self.ATK_02Active` true)
          (`KismetSystemLibrary.Delay` 0.7)
          (set `self.ATK_02Active` false))))))

(fn `ClearTarget`
  (`BlackboardComponent.ClearValue` (`AIBlueprintHelperLibrary.GetBlackboard` (`self.GetController` self)) "Target"))

(fn `GetTarget`
  (returns (Target :type "Actor Object Reference"))
  (return (cast `Actor` (`BlackboardComponent.GetValueAsObject` (`AIBlueprintHelperLibrary.GetBlackboard` (`self.GetController` self)) "Target") :!pure true)))

(fn `SetTarget`
  (params (NewTarget :type "Actor Object Reference"))
  (`BlackboardComponent.SetValueAsObject` (`AIBlueprintHelperLibrary.GetBlackboard` (`AIBlueprintHelperLibrary.GetAIController` self)) "Target" NewTarget))

(fn `UserConstructionScript`)