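; BP_AttackBase is a boss sword attack actor that damages whatever its mesh hits, then destroys itself.
; On spawn it yaws toward the player while a timeline fades the sword in via a material mask, then waits a charge delay.
; It then rotates the mesh, stops tracking, swings the root down with a camera shake, and dither-fades out before destruction.
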(event `self.ReceiveBeginPlay`
  (`self.Charge` 0.0))

(event `self.ReceiveTick`
  (params (DeltaSeconds :type "Float (single-precision)"))
  (bind (_returnvalue_roll _returnvalue_pitch _returnvalue_yaw) (`KismetMathLibrary.BreakRotator` (`KismetMathLibrary.FindLookAtRotation` (`self.K2_GetActorLocation`) (`self.K2_GetActorLocation` (`GameplayStatics.GetPlayerCharacter` 0)))))
  (`self.K2_SetActorRotation` (`KismetMathLibrary.MakeRotator` 0.0 0.0 _returnvalue_yaw)))

(event `Charge`
  (params (ChargeDelay :type "Float (double-precision)"))
  (set `self.Charge Delay` ChargeDelay)
  (`self.FadeIn`))

(event `FadeIn`
  ;[1 1 1] 코멘트
  (bind (_direction _mask) (`Timeline|FadeInSword`)
    (:`Update`
      (`MeshComponent.SetScalarParameterValueOnMaterials` (`self.StaticMesh`) "Mask" _mask))
    (:`Finished`
      (`KismetSystemLibrary.Delay` (`self.Charge Delay`))
      (`self.LaunchAttack`))))

(event `LaunchAttack`
  (bind (_returnvalue_roll _returnvalue_pitch _returnvalue_yaw) (`KismetMathLibrary.BreakRotator` (`self.K2_GetActorRotation`)))
  (bind _staticmesh (`self.StaticMesh`))
  ;[1 1 1] 코멘트
  (`KismetSystemLibrary.MoveComponentTo` _staticmesh (`SceneComponent.RelativeLocation` _staticmesh) (struct :`Yaw` 180.0 :`Roll` 180.0) true true)
  (`KismetSystemLibrary.Delay` 0.2)
  (`self.SetActorTickEnabled` false)
  (`KismetSystemLibrary.MoveComponentTo` (`self.DefaultSceneRoot`) (`self.K2_GetActorLocation`) (`KismetMathLibrary.MakeRotator` _returnvalue_roll -90.0 _returnvalue_yaw) true true)
  (`GameplayStatics.PlayWorldCameraShake` "/Game/MyAssets/Boss/CameraShake_Attack.CameraShake_Attack_C" (`self.K2_GetActorLocation`) 500.0 5000.0)
  (`KismetSystemLibrary.Delay` 1.0)
  (`self.Fade Out`))

(event `self.StaticMesh.OnComponentHit`
  (params (HitComponent :type "PrimitiveComponent Object Reference") (OtherActor :type "Actor Object Reference") (OtherComp :type "PrimitiveComponent Object Reference") (NormalImpulse :type "Vector Structure") (Hit :type "HitResult Structure (by ref)"))
  (`GameplayStatics.ApplyDamage` OtherActor 1.0))

(event `Fade Out`
  (bind (_direction _dither) (`Timeline|DitherFade`)
    (:`Update`
      (`MeshComponent.SetScalarParameterValueOnMaterials` (`self.StaticMesh`) "Alpha Threshold (S)" _dither))
    (:`Finished`
      (`self.K2_DestroyActor`))))

(fn `UserConstructionScript`)